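; BP_Nier is the player character Blueprint, handling Enhanced Input for camera-relative movement and katana attacks.
; Attack input sets an Attacking state on StateComp and calls CombatComp, while moving outside that state stops the current montage.
; Move start and release play and reverse a timeline driving camera lag speed and FOV, though both lerps currently have identical endpoints.
; Left Ctrl only sets a flag, and debug prints remain.
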(event `self.ReceiveTick`
  (params (DeltaSeconds :type "Float (single-precision)")))

(event `EnhancedInput|/Game/Blueprints/Input/Actions/IA_Attack`
  (params (ActionValue :type Boolean) (ElapsedSeconds :type "Float (double-precision)") (TriggeredSeconds :type "Float (double-precision)") (InputAction :type "InputAction Object Reference" :default "/Game/Blueprints/Input/Actions/IA_Attack.IA_Attack"))
  (:`Started`
    (if (not (== (`StateComponent.GetCurrentState` (`self.StateComp`)) (struct :`TagName` "Character.State.Attacking")))
      (`StateComponent.SetState` (`self.StateComp`) (struct :`TagName` "Character.State.Attacking"))
      (`CombatComponent.KatanaAttack` (`self.CombatComp`))
      (set `self.bIsCombatEnabled` true))))

(event `EnhancedInput|/Game/Blueprints/Input/Actions/IA_Move`
  (params (ActionValue :type "Vector2D Structure") (ElapsedSeconds :type "Float (double-precision)") (TriggeredSeconds :type "Float (double-precision)") (InputAction :type "InputAction Object Reference" :default "/Game/Blueprints/Input/Actions/IA_Move.IA_Move"))
  (bind (_returnvalue_roll _returnvalue_pitch _returnvalue_yaw) (`KismetMathLibrary.BreakRotator` (`self.GetControlRotation`)))
  (bind (_returnvalue_roll_2 _returnvalue_pitch_2 _returnvalue_yaw_2) (`KismetMathLibrary.BreakRotator` (`self.GetControlRotation`)))
  ;[1 1 1] Comment
  (:`Triggered`
    (set `self.MoveElapsedSec` ElapsedSeconds)
    (`self.AddMovementInput` (`KismetMathLibrary.GetRightVector` (`KismetMathLibrary.MakeRotator` 0.0 0.0 _returnvalue_yaw_2)) ActionValue_X)
    (`self.AddMovementInput` (`KismetMathLibrary.GetForwardVector` (`KismetMathLibrary.MakeRotator` 0.0 0.0 _returnvalue_yaw)) ActionValue_Y)
    (if (not (== (`StateComponent.GetCurrentState` (`self.StateComp`)) (struct :`TagName` "Character.State.Attacking")))
      (`self.StopAnimMontage` null)))
  (:`Started`
    (`self.HasDirectionalInputEvent`))
  (:`Canceled`
    (`self.ReleaseDirectionalInputEvent` :!label _label)
    (set `self.bIsDoubleClicked` false))
  (:`Completed`
    (goto _label)))

(event `Key|LeftControl`
  (params (Key :type "Key Structure"))
  (:`Pressed`
    (set `self.bIsPressingLeftCtrl` true))
  (:`Released`
    (set `self.bIsPressingLeftCtrl` false)))

(event `EnhancedInput|/Game/Blueprints/Input/Actions/IA_DoubleClick_W`
  (params (ActionValue :type Boolean) (ElapsedSeconds :type "Float (double-precision)") (TriggeredSeconds :type "Float (double-precision)") (InputAction :type "InputAction Object Reference" :default "/Game/Blueprints/Input/Actions/IA_DoubleClick_W.IA_DoubleClick_W")))

(event `EnhancedInput|/Game/Blueprints/Input/Actions/IA_DoubleClick_A`
  (params (ActionValue :type Boolean) (ElapsedSeconds :type "Float (double-precision)") (TriggeredSeconds :type "Float (double-precision)") (InputAction :type "InputAction Object Reference" :default "/Game/Blueprints/Input/Actions/IA_DoubleClick_A.IA_DoubleClick_A")))

(event `EnhancedInput|/Game/Blueprints/Input/Actions/IA_DoubleClick_S`
  (params (ActionValue :type Boolean) (ElapsedSeconds :type "Float (double-precision)") (TriggeredSeconds :type "Float (double-precision)") (InputAction :type "InputAction Object Reference" :default "/Game/Blueprints/Input/Actions/IA_DoubleClick_S.IA_DoubleClick_S")))

(event `EnhancedInput|/Game/Blueprints/Input/Actions/IA_DoubleClick_D`
  (params (ActionValue :type Boolean) (ElapsedSeconds :type "Float (double-precision)") (TriggeredSeconds :type "Float (double-precision)") (InputAction :type "InputAction Object Reference" :default "/Game/Blueprints/Input/Actions/IA_DoubleClick_D.IA_DoubleClick_D")))

(event `HasDirectionalInputEvent`
  (set `self.HasMovementInput` true)
  (`/Engine/EditorBlueprintResources/StandardMacros.DoOnce` false :!label _label
    (:`Completed`
      (bind (_direction _lagspeed) (`Timeline|Timeline` :!label _label_2)
        (:`Update`
          (`|ExecutionSequence`
            (:`then_0`
              (bind _output_get (set `SpringArmComponent.CameraLagSpeed` (`KismetMathLibrary.Lerp` 8.0 8.0 _lagspeed) (`self.CameraBoom`)))
              (`KismetSystemLibrary.PrintString` (`KismetStringLibrary.Concat_StrStr` "Camera Lag Speed：" (`KismetStringLibrary.Conv_DoubleToString` _output_get)) true true (struct :`G` 0.66 :`B` 1.0 :`A` 1.0) 2.0 "Camera Lag Speed"))
            (:`then_1`
              (`CameraComponent.SetFieldOfView` (`self.FollowCamera`) (`KismetMathLibrary.Lerp` 90.0 90.0 _lagspeed)))))))))

(event `ReleaseDirectionalInputEvent`
  (set `self.HasMovementInput` false)
  (`|ExecutionSequence`
    (:`then_0`
      (goto _label :!via `Reset`))
    (:`then_1`
      (goto _label_2 :!via `Reverse`))))

(fn `UserConstructionScript`)