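; An Enhanced Input custom trigger that detects a double click or double press on an input action.
; UpdateState runs the parent update, then timestamps the first update using the owning player controller's game time.
; Within the max double-click time, a zero held duration marks a key release, and the following update returns Triggered.
; Triggering or exceeding the time window resets the state for the next attempt.
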(fn `UpdateState`
  (params (PlayerInput :type "EnhancedPlayerInput Object Reference") (ModifiedValue :type "InputActionValue Structure") (DeltaTime :type "Float (single-precision)"))
  (returns (ReturnValue :type "ETriggerState Enum"))
  (`parent.UpdateState` PlayerInput ModifiedValue DeltaTime)
  (if (`self.bIsFirstTrigger`)
    (set `self.bIsFirstTrigger` false)
    (set `self.SaveTime` (`Actor.GetGameTimeSinceCreation` (`PlayerInput.GetOuterAPlayerController` (`local.PlayerInput`))))
    (elif (<= (- (`Actor.GetGameTimeSinceCreation` (`PlayerInput.GetOuterAPlayerController` (`local.PlayerInput`))) (`self.SaveTime`)) (`self.MaxDoubleClickTime`))
      (if (`self.KeyRelease`)
        (set `self.bIsFirstTrigger` true)
        (set `self.KeyRelease` false)
        (return "Triggered")
        (else
          (set `self.KeyRelease` (== (`self.HeldDuration`) 0.0))))
      (else
        (set `self.bIsFirstTrigger` true)
        (set `self.KeyRelease` false)
        (return "None")))))